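; BP_Tower is a tower actor that reacts with effects when a FlyingCharacter overlaps its goal trigger or its mesh.
; Entering the Box activates the NsGoal effect and deactivates NsRing, then timed delays switch NsGoal off and deactivate NsRing again.
; Overlapping the StaticMesh spawns an explosion emitter at the character's location, with no damage or other gameplay logic.
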(event `self.Box.OnComponentBeginOverlap`
  (params (OverlappedComponent :type "PrimitiveComponent Object Reference") (OtherActor :type "Actor Object Reference") (OtherComp :type "PrimitiveComponent Object Reference") (OtherBodyIndex :type Integer) (bFromSweep :type Boolean) (SweepResult :type "HitResult Structure (by ref)"))
  (bind _ns_goal (`self.Ns_Goal`))
  (cast `FlyingCharacter` OtherActor)
  (`ActorComponent.Activate` _ns_goal false)
  (`ActorComponent.Deactivate` (`self.Ns_Ring`))
  (`KismetSystemLibrary.Delay` 2.0)
  (`ActorComponent.Deactivate` _ns_goal)
  (`KismetSystemLibrary.Delay` 2.0)
  (`ActorComponent.Deactivate` (`self.Ns_Ring`)))

(event `self.StaticMesh.OnComponentBeginOverlap`
  (params (OverlappedComponent :type "PrimitiveComponent Object Reference") (OtherActor :type "Actor Object Reference") (OtherComp :type "PrimitiveComponent Object Reference") (OtherBodyIndex :type Integer) (bFromSweep :type Boolean) (SweepResult :type "HitResult Structure (by ref)"))
  (bind _asflying_character (cast `FlyingCharacter` OtherActor))
  (`GameplayStatics.SpawnEmitterAtLocation` "/Game/StarterContent/Particles/P_Explosion.P_Explosion" (`self.K2_GetActorLocation` _asflying_character)))

(fn `UserConstructionScript`)